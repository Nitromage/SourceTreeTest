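; Moving platform Blueprint meant to slide a static mesh sideways along world Y, though its movement logic is never triggered.
; BeginPlay only stores the mesh's starting world location.
; The disconnected timeline logic would lerp the mesh 400 units along +Y from that point with a swept move.
; Its Finished output loops into a switch on timeline direction that restarts playback from the start or reverses from the end.
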(event `self.ReceiveBeginPlay`
  ;[1 1 1] Platform Movement Y-axis
  (bind _output_get (set `self.Init Loc` (`SceneComponent.K2_GetComponentLocation` (`self.StaticMeshComponent`)))))

(fn `UserConstructionScript`)