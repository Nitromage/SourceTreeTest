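; PuzzlePlate is a plate actor that sinks slightly and plays a click sound when another actor overlaps it.
; BeginPlay stores the mesh's start position, and overlap sets IsOn, which this graph never clears.
; Tick snaps the mesh to the lowered or original position every frame according to IsOn, without interpolation.
; An Invalid_Action sound node is present but never runs.
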(event `self.ReceiveBeginPlay`
  (set `self.StartPosition` (`SceneComponent.K2_GetComponentLocation` (`self.StaticMesh`))))

(event `self.ReceiveActorBeginOverlap`
  (params (OtherActor :type "Actor Object Reference"))
  (set `self.IsOn` true)
  (`GameplayStatics.PlaySoundAtLocation` "/Engine/VREditor/Sounds/UI/Gizmo_Handle_Clicked.Gizmo_Handle_Clicked" (`self.K2_GetActorLocation`)))

(event `self.ReceiveTick`
  (params (DeltaSeconds :type "Float (single-precision)"))
  (bind _staticmesh (`self.StaticMesh`))
  (bind (_startposition_x _startposition_y _startposition_z) (`KismetMathLibrary.BreakVector` (`self.StartPosition`)))
  (if (`self.IsOn`)
    (`SceneComponent.K2_SetWorldLocation` _staticmesh (`KismetMathLibrary.MakeVector` _startposition_x _startposition_y (+ _startposition_z -5.0)) false false)
    (else
      (`SceneComponent.K2_SetWorldLocation` _staticmesh (`self.StartPosition`) false false))))

(fn `UserConstructionScript`)