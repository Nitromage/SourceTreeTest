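; Rock hazard that damages and knocks back the third-person character on overlap, then destroys itself.
; The hit subtracts 10 from PlayerHealth and zeroes player 0's velocity before launching the character.
; The velocity-change impulse points horizontally away from a referenced Center actor, based on the rock's position, with added upward lift.
; An unconnected branch for a weaker impulse while falling never runs.
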(event `self.ReceiveActorBeginOverlap`
  (params (OtherActor :type "Actor Object Reference"))
  (bind (_returnvalue_x _returnvalue_y _returnvalue_z) (`KismetMathLibrary.BreakVector` (`self.K2_GetActorLocation`)))
  (bind (_impulse_x _impulse_y _impulse_z) (`KismetMathLibrary.BreakVector` (`self.Impulse`)))
  (bind (_returnvalue_x_2 _returnvalue_y_2) (`KismetMathLibrary.BreakVector` (`self.K2_GetActorLocation` (`self.Center`))))
  (bind _asthird_person_character (cast `/Game/ThirdPersonBP/Blueprints/ThirdPersonCharacter` OtherActor))
  (set `self.Impulse` (`KismetMathLibrary.Normal` (- (`KismetMathLibrary.MakeVector` _returnvalue_x_2 _returnvalue_y_2 _returnvalue_z) (`KismetMathLibrary.MakeVector` _returnvalue_x _returnvalue_y _returnvalue_z))))
  (set `/Game/ThirdPersonBP/Blueprints/ThirdPersonCharacter.PlayerHealth` (- (`/Game/ThirdPersonBP/Blueprints/ThirdPersonCharacter.PlayerHealth` _asthird_person_character) 10) _asthird_person_character)
  (set `MovementComponent.Velocity` (0.0 0.0 0.0) (`Pawn.GetMovementComponent` (`GameplayStatics.GetPlayerCharacter` 0)))
  (set `self.Impulse` (* (`KismetMathLibrary.MakeVector` _impulse_x _impulse_y (+ -1.0 _impulse_z)) -1000))
  (`CharacterMovementComponent.AddImpulse` (`Character.CharacterMovement` _asthird_person_character) (`self.Impulse`) true)
  (`self.K2_DestroyActor`))

(fn `UserConstructionScript`)