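; ClearGameCollectable is a spinning star pickup that ends a level by returning the player to Map_HubWorld when overlapped.
; On BeginPlay it loads its ID through StarScript if the test save slot exists.
; On overlap it saves the ID, plays a sound, destroys itself, increments TotalStars on MyGameinstance and opens the hub.
; A bobbing timeline exists but is never triggered.
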(event `self.ReceiveBeginPlay`
  (bind _returnvalue (`GameplayStatics.DoesSaveGameExist` "TestSaveSlot"))
  (if _returnvalue
    (`StarScript.LoadIDTest` (`self.StarScript`))))

(event `self.ReceiveActorBeginOverlap`
  (params (OtherActor :type "Actor Object Reference"))
  ;[1 1 1] On Collect
  (bind _returnvalue (`GameplayStatics.DoesSaveGameExist` "TestSaveSlot"))
  (`StarScript.SaveIDTest` (`self.StarScript`) _returnvalue)
  (`GameplayStatics.PlaySoundAtLocation` "/Game/Levels/Sound/337049_shinephoenixstormcrow_320655-rhodesmas-lev.337049_shinephoenixstormcrow_320655-rhodesmas-lev" (`self.K2_GetActorLocation`))
  (`self.K2_DestroyActor`)
  (bind _asmy_gameinstance (cast `/Game/Levels/MyGameinstance` (`GameplayStatics.GetGameInstance`)))
  (bind _output_get (set `/Game/Levels/MyGameinstance.TotalStars` (+ (`/Game/Levels/MyGameinstance.TotalStars` _asmy_gameinstance) 1) _asmy_gameinstance))
  (`KismetSystemLibrary.PrintString` (`KismetStringLibrary.Conv_IntToString` _output_get))
  (`GameplayStatics.OpenLevel` "Map_HubWorld"))

(event `self.ReceiveTick`
  (params (DeltaSeconds :type "Float (single-precision)"))
  ;[1 1 1] movement
  (`self.K2_AddActorLocalRotation` (struct :`Yaw` 3.0)))

(fn `UserConstructionScript`)