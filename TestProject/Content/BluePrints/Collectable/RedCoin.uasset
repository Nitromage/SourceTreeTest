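; RedCoin is a collectable coin actor that the ThirdPersonCharacter picks up by overlapping it.
; On pickup it plays a sound, destroys itself, increments TotalCoin on MyGameinstance and prints the new total.
; Each tick it rotates by a fixed yaw step and calls Play on the Coin timeline, whose updates add a local offset to move it.
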(event `self.ReceiveActorBeginOverlap`
  (params (OtherActor :type "Actor Object Reference"))
  ;[1 1 1] On Collect
  (cast `/Game/ThirdPersonBP/Blueprints/ThirdPersonCharacter` OtherActor)
  (`GameplayStatics.PlaySoundAtLocation` "/Game/Levels/Sound/337049_shinephoenixstormcrow_320655-rhodesmas-lev.337049_shinephoenixstormcrow_320655-rhodesmas-lev" (`self.K2_GetActorLocation`))
  (`self.K2_DestroyActor`)
  (bind _asmy_gameinstance (cast `/Game/Levels/MyGameinstance` (`GameplayStatics.GetGameInstance`)))
  (bind _output_get (set `/Game/Levels/MyGameinstance.TotalCoin` (+ (`/Game/Levels/MyGameinstance.TotalCoin` _asmy_gameinstance) 1) _asmy_gameinstance))
  (`KismetSystemLibrary.PrintString` (`KismetStringLibrary.Conv_IntToString` _output_get)))

(event `self.ReceiveTick`
  (params (DeltaSeconds :type "Float (single-precision)"))
  ;[1 1 1] movement
  (`self.K2_AddActorLocalRotation` (struct :`Yaw` 3.0))
  (bind (_direction _coin) (`Timeline|Coin`)
    (:`Update`
      (`self.K2_AddActorLocalOffset` _coin))))

(fn `UserConstructionScript`)