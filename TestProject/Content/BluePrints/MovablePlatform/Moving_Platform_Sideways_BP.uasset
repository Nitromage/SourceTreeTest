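; Moving platform Blueprint meant to slide a static mesh sideways along X, Y or both, over a set Distance.
; BeginPlay only caches the mesh's starting world location.
; A timeline drives a swept lerp from that point, with axis flags choosing the target and X as the fallback, and Finished looping into a direction switch.
; No event reaches that timeline logic, so the platform never moves as wired.
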(event `self.ReceiveBeginPlay`
  ;[1 1 1] Platform Movement
  (if (and (`self.IsYAxis`) (`self.IsXAxis`))
    (bind _output_get (set `self.Init Loc` (`SceneComponent.K2_GetComponentLocation` (`self.StaticMeshComponent`))))
    (elif (`self.IsYAxis`)
      (bind _output_get_2 (set `self.Init Loc` (`SceneComponent.K2_GetComponentLocation` (`self.StaticMeshComponent`))))
      (elif (`self.IsXAxis`)
        (bind _output_get_3 (set `self.Init Loc` (`SceneComponent.K2_GetComponentLocation` (`self.StaticMeshComponent`))))))))

(fn `UserConstructionScript`)