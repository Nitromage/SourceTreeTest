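; BallSpawner is an actor that spawns Rock actors at its own transform while a ThirdPersonCharacter is inside its overlap area, the rock field.
; Overlap events switch it on and off, priming the timer on entry so the first rock appears immediately.
; Tick accumulates time, spawns a rock whenever TimeBetween is exceeded, and passes its Center reference to each new rock.
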(event `self.ReceiveActorEndOverlap`
  (params (OtherActor :type "Actor Object Reference"))
  (cast `/Game/ThirdPersonBP/Blueprints/ThirdPersonCharacter` OtherActor)
  (set `self.IsOn` false)
  (`KismetSystemLibrary.PrintString` "Leaving rock field"))

(event `self.ReceiveActorBeginOverlap`
  (params (OtherActor :type "Actor Object Reference"))
  (cast `/Game/ThirdPersonBP/Blueprints/ThirdPersonCharacter` OtherActor)
  (set `self.IsOn` true)
  (set `self.Timer` (`self.TimeBetween`))
  (`KismetSystemLibrary.PrintString` "Entering rock field"))

(event `self.ReceiveTick`
  (params (DeltaSeconds :type "Float (single-precision)"))
  (if (`self.IsOn`)
    (bind _output_get (set `self.Timer` (+ DeltaSeconds (`self.Timer`))))
    (if (> _output_get (`self.TimeBetween`))
      (set `self.Timer` 0.0)
      (bind _returnvalue (`|SpawnActorFromClass` (`self.Rock`) (`self.GetTransform`) "AlwaysSpawn" "OverrideRootScale" null null))
      (bind _asrock (cast `/Game/BluePrints/RollingBall/Rock` _returnvalue)
        (:`then`
          (set `/Game/BluePrints/RollingBall/Rock.Center` (`self.Center`) _asrock))
        (:`CastFailed`
          (`KismetSystemLibrary.PrintString` "Error setting center object for rock"))))))

(fn `UserConstructionScript`)