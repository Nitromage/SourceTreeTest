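; CountCoins is a collectable-goal actor that reveals a referenced Star once the player's coin total reaches a threshold.
; It hides the Star on BeginPlay, then polls TotalCoin on MyGameinstance against CoinCount every Tick while IsOn is set.
; On reaching the count it unhides the Star, clears IsOn so the reveal fires once, and plays the Cinematic sequence if valid.
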(event `self.ReceiveBeginPlay`
  (`self.SetActorHiddenInGame` (`self.Star`) true))

(event `self.ReceiveTick`
  (params (DeltaSeconds :type "Float (single-precision)"))
  (bind _cinematic (`self.Cinematic`))
  (if (`self.IsOn`)
    (bind _asmy_gameinstance (cast `/Game/Levels/MyGameinstance` (`GameplayStatics.GetGameInstance`)))
    (if (>= (`/Game/Levels/MyGameinstance.TotalCoin` _asmy_gameinstance) (`self.CoinCount`))
      (`self.SetActorHiddenInGame` (`self.Star`) false)
      (set `self.IsOn` false)
      (`/Engine/EditorBlueprintResources/StandardMacros.IsValid` _cinematic
        (:`Is Valid`
          (`MovieSceneSequencePlayer.Play` (`LevelSequenceActor.SequencePlayer` _cinematic)))))))

(fn `UserConstructionScript`)