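; BouncePad is an actor that launches an overlapping ThirdPersonCharacter and deducts Damage from its health if that is above zero.
; On overlap it disables the character's CanMove and applies a velocity-change impulse of velocity times BounceFactor, substituting a downward component before scaling when vertical speed is zero.
; Tick restores CanMove on the last stored character once it is no longer falling.
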(event `self.ReceiveTick`
  (params (DeltaSeconds :type "Float (single-precision)"))
  (bind _player (`self.Player`))
  (`/Engine/EditorBlueprintResources/StandardMacros.IsValid` _player
    (:`Is Valid`
      (if (not (`/Game/ThirdPersonBP/Blueprints/ThirdPersonCharacter.CanMove` _player))
        (if (not (`NavMovementComponent.IsFalling` (`Character.CharacterMovement` (`self.Player`))))
          (set `/Game/ThirdPersonBP/Blueprints/ThirdPersonCharacter.CanMove` true (`self.Player`)))))))

(event `self.ReceiveActorBeginOverlap`
  (params (OtherActor :type "Actor Object Reference"))
  (bind _player (`self.Player`))
  (bind (_returnvalue_x _returnvalue_y _returnvalue_z) (`KismetMathLibrary.BreakVector` (`self.GetVelocity` (`self.Player`))))
  (bind (_returnvalue_x_2 _returnvalue_y_2 _returnvalue_z_2) (`KismetMathLibrary.BreakVector` (`self.GetVelocity` (`self.Player`))))
  (bind _playerhealth (`/Game/ThirdPersonBP/Blueprints/ThirdPersonCharacter.PlayerHealth` _player))
  (bind _asthird_person_character (cast `/Game/ThirdPersonBP/Blueprints/ThirdPersonCharacter` OtherActor))
  (set `/Game/ThirdPersonBP/Blueprints/ThirdPersonCharacter.CanMove` false _asthird_person_character)
  (set `self.Player` _asthird_person_character)
  (if (!= _returnvalue_z 0.0)
    (set `self.Impulse` (* (`self.GetVelocity` (`self.Player`)) (`self.BounceFactor`)))
    (else
      (set `self.Impulse` (* (+ (0.0 0.0 0.0) (`KismetMathLibrary.MakeVector` _returnvalue_x_2 _returnvalue_y_2 (+ _returnvalue_z_2 -500.0))) (`self.BounceFactor`)))))
  (`CharacterMovementComponent.AddImpulse` (`Character.CharacterMovement` (`self.Player`)) (`self.Impulse`) true)
  (if (> _playerhealth 0)
    (set `/Game/ThirdPersonBP/Blueprints/ThirdPersonCharacter.PlayerHealth` (- _playerhealth (`self.Damage`)) _player)))

(fn `UserConstructionScript`)